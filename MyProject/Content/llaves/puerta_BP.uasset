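; Door Blueprint that opens only once all collectables are picked up.
; A Box overlap enables input for the first-person character, and the interac action checks CollectablesLeft on the GameMode.
; At zero, the Cronograma timeline swings StaticMesh open by yaw; otherwise a Tefalta widget is shown.
; Cronograma_0 is also reversed, but the StaticMesh1 rotation using it is disconnected and never runs.
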(event `self.Box.OnComponentBeginOverlap`
  (params (OverlappedComponent :type "PrimitiveComponent Object Reference") (OtherActor :type "Actor Object Reference") (OtherComp :type "PrimitiveComponent Object Reference") (OtherBodyIndex :type Integer) (bFromSweep :type Boolean) (SweepResult :type "HitResult Structure (by ref)"))
  (cast `/Game/FirstPerson/Blueprints/BP_FirstPersonCharacter` OtherActor)
  (`self.EnableInput` (`GameplayStatics.GetPlayerController` 0)))

(event `self.Box.OnComponentEndOverlap`
  (params (OverlappedComponent :type "PrimitiveComponent Object Reference") (OtherActor :type "Actor Object Reference") (OtherComp :type "PrimitiveComponent Object Reference") (OtherBodyIndex :type Integer))
  (cast `/Game/FirstPerson/Blueprints/BP_FirstPersonCharacter` OtherActor)
  (`self.DisableInput` (`GameplayStatics.GetPlayerController` 0)))

(event `InputAction|interac`
  (params (Key :type "Key Structure"))
  (:`Pressed`
    (bind _asbp_first_person_game_mode (cast `/Game/FirstPerson/Blueprints/BP_FirstPersonGameMode` (`GameplayStatics.GetGameMode`)))
    (if (== (`/Game/FirstPerson/Blueprints/BP_FirstPersonGameMode.collectables Left` _asbp_first_person_game_mode) 0)
      (`|ExecutionSequence`
        (:`then_0`
          (bind (_direction _pista_nueva_0) (`Timeline|Cronograma`)
            (:`Update`
              (`SceneComponent.K2_SetRelativeRotation` (`self.StaticMesh`) (`KismetMathLibrary.MakeRotator` 0.0 0.0 (`KismetMathLibrary.Lerp` 0.0 -90.0 _pista_nueva_0)) false false))))
        (:`then_1`
          (bind (_direction_2 _pista_nueva_0_2) (`Timeline|Cronograma_0` :!via `Reverse`))))
      (else
        (bind _returnvalue (`|CreateWidget` "/Game/llaves/tefalta.tefalta_C"))
        (`UserWidget.AddToViewport` _returnvalue 0)))))

(fn `UserConstructionScript`)